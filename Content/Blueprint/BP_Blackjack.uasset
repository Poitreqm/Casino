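; BP_Blackjack is an interactable blackjack actor that lets the player take a position at it with a key press.
; BeginPlay caches the third-person character, enables input on the actor and turns on mouse-over and click events.
; Box overlap toggles a usability flag, without filtering the overlapping actor.
; While flagged, pressing B calls the character's blackjack camera function and snaps it to a fixed offset and zero rotation.
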(event OnComponentBeginOverlap(Box)
  (params (OverlappedComponent :type Primitive%20Component%20Object%20Reference) (OtherActor :type Actor%20Object%20Reference) (OtherComp :type Primitive%20Component%20Object%20Reference) (OtherBodyIndex :type Integer) (bFromSweep :type Boolean) (SweepResult :type Hit%20Result%20Structure%20%28by%20ref%29))
  (Variables|Default|SetcanUseBlackjack true)
  (Development|PrintString "Hello"))

(event OnComponentEndOverlap(Box)
  (params (OverlappedComponent :type Primitive%20Component%20Object%20Reference) (OtherActor :type Actor%20Object%20Reference) (OtherComp :type Primitive%20Component%20Object%20Reference) (OtherBodyIndex :type Integer))
  (Variables|Default|SetcanUseBlackjack false))

(event EventBeginPlay
  (bind _asbp_third_person_character (Utilities|Casting|CastToBP_ThirdPersonCharacter (Game|Player|GetPlayerPawn 0)))
  (Variables|Default|SetPlayerCharacter _asbp_third_person_character)
  ;[1 1 1] включаем возможность нажимать кнопки на клавиатуре
  (Input|EnableInput (Game|GetPlayerController 0))
  ;[1 1 1] включаем возможность исспользовать мышку
  (Variables|/Script/Engine.PlayerController|SetbEnableMouseOverEvents (Game|GetPlayerController 0) true)
  ;[1 1 1] включаем возможность исспользовать клик
  (Variables|/Script/Engine.PlayerController|SetbEnableClickEvents (Game|GetPlayerController 0) true))

(event Collision|EventActorBeginOverlap
  (params (OtherActor :type Actor%20Object%20Reference)))

(event EventTick
  (params (DeltaSeconds :type Float%20%28single-precision%29)))

(event Input|KeyboardEvents|B
  (params (Key :type Key%20Structure :default "None"))
  (bind _playercharacter (Variables|Default|GetPlayerCharacter))
  (:Pressed
    (if (Variables|Default|GetcanUseBlackjack)
      (Default|GetCameraBlackjack (Variables|Default|GetPlayerCharacter))
      (Transformation|AddActorWorldOffset _playercharacter (Utilities|Operators|Subtract (Transformation|GetActorLocation) (Transformation|GetActorLocation _playercharacter) "150.000000,0.000000,0.000000"))
      (Transformation|SetActorRelativeRotation _playercharacter))))

(fn ConstructionScript)