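; Playing card actor that picks a random face and point value, with blackjack-like scoring.
; The Construction Script rolls one of 52 cases, sets the matching suit and rank material on Plane, and adds the rank's points to its own CardPoint variable.
; Face cards and aces add 10, and an ace drops to 1 if CardPoint exceeds 21.
; Each roll is independent, with no deck tracking to prevent duplicates.
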(fn ConstructionScript
  (bind _plane (Variables|Default|GetPlane))
  (bind _plane_2 (Variables|Default|GetPlane))
  (bind _plane_3 (Variables|Default|GetPlane))
  (bind _plane_4 (Variables|Default|GetPlane))
  (switch int (Math|Random|RandomIntegerinRange 0 51)
    (:0
      ;[1 1 1] крести
      (Rendering|Material|SetMaterial _plane_2 0 "/Game/Textures/T_Club_2_Mat.T_Club_2_Mat")
      ;[1 1 1] за каждую карту даются очки
      (Variables|Default|SetcardPoint (+ (Variables|Default|GetcardPoint) 2)))
    (:1
      (Rendering|Material|SetMaterial _plane_2 0 "/Game/Textures/T_Club_3_Mat.T_Club_3_Mat")
      (Variables|Default|SetcardPoint (+ (Variables|Default|GetcardPoint) 3)))
    (:2
      (Rendering|Material|SetMaterial _plane_2 0 "/Game/Textures/T_Club_4_Mat.T_Club_4_Mat")
      (Variables|Default|SetcardPoint (+ (Variables|Default|GetcardPoint) 4)))
    (:3
      (Rendering|Material|SetMaterial _plane_2 0 "/Game/Textures/T_Club_5_Mat.T_Club_5_Mat")
      (Variables|Default|SetcardPoint (+ (Variables|Default|GetcardPoint) 5)))
    (:4
      (Rendering|Material|SetMaterial _plane_2 0 "/Game/Textures/T_Club_6_Mat.T_Club_6_Mat")
      (Variables|Default|SetcardPoint (+ (Variables|Default|GetcardPoint) 6)))
    (:5
      (Rendering|Material|SetMaterial _plane_2 0 "/Game/Textures/T_Club_7_Mat.T_Club_7_Mat")
      (Variables|Default|SetcardPoint (+ (Variables|Default|GetcardPoint) 7)))
    (:6
      (Rendering|Material|SetMaterial _plane_2 0 "/Game/Textures/T_Club_8_Mat.T_Club_8_Mat")
      (Variables|Default|SetcardPoint (+ (Variables|Default|GetcardPoint) 8)))
    (:7
      (Rendering|Material|SetMaterial _plane_2 0 "/Game/Textures/T_Club_9_Mat.T_Club_9_Mat")
      (Variables|Default|SetcardPoint (+ (Variables|Default|GetcardPoint) 9)))
    (:8
      (Rendering|Material|SetMaterial _plane_2 0 "/Game/Textures/T_Club_10_Mat.T_Club_10_Mat")
      (Variables|Default|SetcardPoint (+ (Variables|Default|GetcardPoint) 10)))
    (:9
      (Rendering|Material|SetMaterial _plane_2 0 "/Game/Textures/T_Club_Jack_Mat.T_Club_Jack_Mat")
      (Variables|Default|SetcardPoint (+ (Variables|Default|GetcardPoint) 10)))
    (:10
      (Rendering|Material|SetMaterial _plane_2 0 "/Game/Textures/T_Club_Queen_Mat.T_Club_Queen_Mat")
      (Variables|Default|SetcardPoint (+ (Variables|Default|GetcardPoint) 10)))
    (:11
      (Rendering|Material|SetMaterial _plane_2 0 "/Game/Textures/T_Club_King_Mat.T_Club_King_Mat")
      (Variables|Default|SetcardPoint (+ (Variables|Default|GetcardPoint) 10)))
    (:12
      (Rendering|Material|SetMaterial _plane_2 0 "/Game/Textures/T_Club_Ace_Mat.T_Club_Ace_Mat")
      (Variables|Default|SetcardPoint (+ (Variables|Default|GetcardPoint) 10))
      ;[1 1 1] если приходит туз то дается 1 очко а не 10
      (if (> (Variables|Default|GetcardPoint) 21)
        (Variables|Default|SetcardPoint (- (Variables|Default|GetcardPoint) 9))))
    (:13
      ;[1 1 1] пики
      (Rendering|Material|SetMaterial _plane 0 "/Game/Textures/T_Spade_2_Mat.T_Spade_2_Mat")
      (Variables|Default|SetcardPoint (+ (Variables|Default|GetcardPoint) 2)))
    (:14
      (Rendering|Material|SetMaterial _plane 0 "/Game/Textures/T_Spade_3_Mat.T_Spade_3_Mat")
      (Variables|Default|SetcardPoint (+ (Variables|Default|GetcardPoint) 3)))
    (:15
      (Rendering|Material|SetMaterial _plane 0 "/Game/Textures/T_Spade_4_Mat.T_Spade_4_Mat")
      (Variables|Default|SetcardPoint (+ (Variables|Default|GetcardPoint) 4)))
    (:16
      (Rendering|Material|SetMaterial _plane 0 "/Game/Textures/T_Spade_5_Mat.T_Spade_5_Mat")
      (Variables|Default|SetcardPoint (+ (Variables|Default|GetcardPoint) 5)))
    (:17
      (Rendering|Material|SetMaterial _plane 0 "/Game/Textures/T_Spade_6_Mat.T_Spade_6_Mat")
      (Variables|Default|SetcardPoint (+ (Variables|Default|GetcardPoint) 6)))
    (:18
      (Rendering|Material|SetMaterial _plane 0 "/Game/Textures/T_Spade_7_Mat.T_Spade_7_Mat")
      (Variables|Default|SetcardPoint (+ (Variables|Default|GetcardPoint) 7)))
    (:19
      (Rendering|Material|SetMaterial _plane 0 "/Game/Textures/T_Spade_8_Mat.T_Spade_8_Mat")
      (Variables|Default|SetcardPoint (+ (Variables|Default|GetcardPoint) 8)))
    (:20
      (Rendering|Material|SetMaterial _plane 0 "/Game/Textures/T_Spade_9_Mat.T_Spade_9_Mat")
      (Variables|Default|SetcardPoint (+ (Variables|Default|GetcardPoint) 9)))
    (:21
      (Rendering|Material|SetMaterial _plane 0 "/Game/Textures/T_Spade_10_Mat.T_Spade_10_Mat")
      (Variables|Default|SetcardPoint (+ (Variables|Default|GetcardPoint) 10)))
    (:22
      (Rendering|Material|SetMaterial _plane 0 "/Game/Textures/T_Spade_Jack_Mat.T_Spade_Jack_Mat")
      (Variables|Default|SetcardPoint (+ (Variables|Default|GetcardPoint) 10)))
    (:23
      (Rendering|Material|SetMaterial _plane 0 "/Game/Textures/T_Spade_Queen_Mat.T_Spade_Queen_Mat")
      (Variables|Default|SetcardPoint (+ (Variables|Default|GetcardPoint) 10)))
    (:24
      (Rendering|Material|SetMaterial _plane 0 "/Game/Textures/T_Spade_King_Mat.T_Spade_King_Mat")
      (Variables|Default|SetcardPoint (+ (Variables|Default|GetcardPoint) 10)))
    (:25
      (Rendering|Material|SetMaterial _plane 0 "/Game/Textures/T_Spade_Ace_Mat.T_Spade_Ace_Mat")
      (Variables|Default|SetcardPoint (+ (Variables|Default|GetcardPoint) 10))
      ;[1 1 1] если приходит туз то дается 1 очко а не 10
      (if (> (Variables|Default|GetcardPoint) 21)
        (Variables|Default|SetcardPoint (- (Variables|Default|GetcardPoint) 9))))
    (:26
      ;[1 1 1] бубна
      (Rendering|Material|SetMaterial _plane_3 0 "/Game/Textures/T_Diamond_2_Mat.T_Diamond_2_Mat")
      (Variables|Default|SetcardPoint (+ (Variables|Default|GetcardPoint) 2)))
    (:27
      (Rendering|Material|SetMaterial _plane_3 0 "/Game/Textures/T_Diamond_3_Mat.T_Diamond_3_Mat")
      (Variables|Default|SetcardPoint (+ (Variables|Default|GetcardPoint) 3)))
    (:28
      (Rendering|Material|SetMaterial _plane_3 0 "/Game/Textures/T_Diamond_4_Mat.T_Diamond_4_Mat")
      (Variables|Default|SetcardPoint (+ (Variables|Default|GetcardPoint) 4)))
    (:29
      (Rendering|Material|SetMaterial _plane_3 0 "/Game/Textures/T_Diamond_5_Mat.T_Diamond_5_Mat")
      (Variables|Default|SetcardPoint (+ (Variables|Default|GetcardPoint) 5)))
    (:30
      (Rendering|Material|SetMaterial _plane_3 0 "/Game/Textures/T_Diamond_6_Mat.T_Diamond_6_Mat")
      (Variables|Default|SetcardPoint (+ (Variables|Default|GetcardPoint) 6)))
    (:31
      (Rendering|Material|SetMaterial _plane_3 0 "/Game/Textures/T_Diamond_7_Mat.T_Diamond_7_Mat")
      (Variables|Default|SetcardPoint (+ (Variables|Default|GetcardPoint) 7)))
    (:32
      (Rendering|Material|SetMaterial _plane_3 0 "/Game/Textures/T_Diamond_8_Mat.T_Diamond_8_Mat")
      (Variables|Default|SetcardPoint (+ (Variables|Default|GetcardPoint) 8)))
    (:33
      (Rendering|Material|SetMaterial _plane_3 0 "/Game/Textures/T_Diamond_9_Mat.T_Diamond_9_Mat")
      (Variables|Default|SetcardPoint (+ (Variables|Default|GetcardPoint) 9)))
    (:34
      (Rendering|Material|SetMaterial _plane_3 0 "/Game/Textures/T_Diamond_10_Mat.T_Diamond_10_Mat")
      (Variables|Default|SetcardPoint (+ (Variables|Default|GetcardPoint) 10)))
    (:35
      (Rendering|Material|SetMaterial _plane_3 0 "/Game/Textures/T_Diamond_Jack_Mat.T_Diamond_Jack_Mat")
      (Variables|Default|SetcardPoint (+ (Variables|Default|GetcardPoint) 10)))
    (:36
      (Rendering|Material|SetMaterial _plane_3 0 "/Game/Textures/T_Diamond_Queen_Mat.T_Diamond_Queen_Mat")
      (Variables|Default|SetcardPoint (+ (Variables|Default|GetcardPoint) 10)))
    (:37
      (Rendering|Material|SetMaterial _plane_3 0 "/Game/Textures/T_Diamond_King_Mat.T_Diamond_King_Mat")
      (Variables|Default|SetcardPoint (+ (Variables|Default|GetcardPoint) 10)))
    (:38
      (Rendering|Material|SetMaterial _plane_3 0 "/Game/Textures/T_Diamond_Ace_Mat.T_Diamond_Ace_Mat")
      (Variables|Default|SetcardPoint (+ (Variables|Default|GetcardPoint) 10))
      ;[1 1 1] если приходит туз то дается 1 очко а не 10
      (if (> (Variables|Default|GetcardPoint) 21)
        (Variables|Default|SetcardPoint (- (Variables|Default|GetcardPoint) 9))))
    (:39
      ;[1 1 1] черви
      (Rendering|Material|SetMaterial _plane_4 0 "/Game/Textures/T_Heart_2_Mat.T_Heart_2_Mat")
      (Variables|Default|SetcardPoint (+ (Variables|Default|GetcardPoint) 2)))
    (:40
      (Rendering|Material|SetMaterial _plane_4 0 "/Game/Textures/T_Heart_3_Mat.T_Heart_3_Mat")
      (Variables|Default|SetcardPoint (+ (Variables|Default|GetcardPoint) 3)))
    (:41
      (Rendering|Material|SetMaterial _plane_4 0 "/Game/Textures/T_Heart_4_Mat.T_Heart_4_Mat")
      (Variables|Default|SetcardPoint (+ (Variables|Default|GetcardPoint) 4)))
    (:42
      (Rendering|Material|SetMaterial _plane_4 0 "/Game/Textures/T_Heart_5_Mat.T_Heart_5_Mat")
      (Variables|Default|SetcardPoint (+ (Variables|Default|GetcardPoint) 5)))
    (:43
      (Rendering|Material|SetMaterial _plane_4 0 "/Game/Textures/T_Heart_6_Mat.T_Heart_6_Mat")
      (Variables|Default|SetcardPoint (+ (Variables|Default|GetcardPoint) 6)))
    (:44
      (Rendering|Material|SetMaterial _plane_4 0 "/Game/Textures/T_Heart_7_Mat.T_Heart_7_Mat")
      (Variables|Default|SetcardPoint (+ (Variables|Default|GetcardPoint) 7)))
    (:45
      (Rendering|Material|SetMaterial _plane_4 0 "/Game/Textures/T_Heart_8_Mat.T_Heart_8_Mat")
      (Variables|Default|SetcardPoint (+ (Variables|Default|GetcardPoint) 8)))
    (:46
      (Rendering|Material|SetMaterial _plane_4 0 "/Game/Textures/T_Heart_9_Mat.T_Heart_9_Mat")
      (Variables|Default|SetcardPoint (+ (Variables|Default|GetcardPoint) 9)))
    (:47
      (Rendering|Material|SetMaterial _plane_4 0 "/Game/Textures/T_Heart_10_Mat.T_Heart_10_Mat")
      (Variables|Default|SetcardPoint (+ (Variables|Default|GetcardPoint) 10)))
    (:48
      (Rendering|Material|SetMaterial _plane_4 0 "/Game/Textures/T_Heart_Jack_Mat.T_Heart_Jack_Mat")
      (Variables|Default|SetcardPoint (+ (Variables|Default|GetcardPoint) 10)))
    (:49
      (Rendering|Material|SetMaterial _plane_4 0 "/Game/Textures/T_Heart_Queen_Mat.T_Heart_Queen_Mat")
      (Variables|Default|SetcardPoint (+ (Variables|Default|GetcardPoint) 10)))
    (:50
      (Rendering|Material|SetMaterial _plane_4 0 "/Game/Textures/T_Heart_King_Mat.T_Heart_King_Mat")
      (Variables|Default|SetcardPoint (+ (Variables|Default|GetcardPoint) 10)))
    (:51
      (Rendering|Material|SetMaterial _plane_4 0 "/Game/Textures/T_Heart_Ace_Mat.T_Heart_Ace_Mat")
      (Variables|Default|SetcardPoint (+ (Variables|Default|GetcardPoint) 10))
      ;[1 1 1] если приходит туз то дается 1 очко а не 10
      (if (> (Variables|Default|GetcardPoint) 21)
        (Variables|Default|SetcardPoint (- (Variables|Default|GetcardPoint) 9))))))