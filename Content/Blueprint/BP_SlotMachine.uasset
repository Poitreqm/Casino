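; Interactive slot machine actor: pressing E inside its trigger box moves the player to the screen and switches to the machine camera.
; Mouse-over lights the button boxes; clicking Spin rotates three reels in random steps on a looping timer, and Cash Out restores the normal camera.
; After the spin, component tags under each reel's check box add symbol-weighted points, whose three-of-a-kind totals decide player credit changes and the red win line.
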(event OnClicked(CashOutBox)
  (params (TouchedComponent :type Primitive%20Component%20Object%20Reference) (ButtonPressed :type Key%20Structure :default "None"))
  (Default|GetNormalCamera (Variables|Default|GetPlayerCharacter))
  (Variables|Default|SetcharacterNowUseMachine false))

(event OnBeginCursorOver(MaxCreditBox)
  (params (TouchedComponent :type Primitive%20Component%20Object%20Reference))
  ;[1 1 1] On Begin Cursor Over работает с Box Collision только если Collision Presets - BlockAllDinamic
  (Rendering|SetVisibility (Variables|Default|GetRectLightMaxCredit) true false))

(event OnEndCursorOver(CashOutBox)
  (params (TouchedComponent :type Primitive%20Component%20Object%20Reference))
  (Rendering|SetVisibility (Variables|Default|GetRectLightCashOut) false false))

(event OnBeginCursorOver(AlarmBox)
  (params (TouchedComponent :type Primitive%20Component%20Object%20Reference))
  (Rendering|SetVisibility (Variables|Default|GetRectLightAlarmBox) true false))

(event OnEndCursorOver(AlarmBox)
  (params (TouchedComponent :type Primitive%20Component%20Object%20Reference))
  (Rendering|SetVisibility (Variables|Default|GetRectLightAlarmBox) false false))

(event OnComponentBeginOverlap(CheckSlotBoxFirstReel)
  (params (OverlappedComponent :type Primitive%20Component%20Object%20Reference) (OtherActor :type Actor%20Object%20Reference) (OtherComp :type Primitive%20Component%20Object%20Reference) (OtherBodyIndex :type Integer) (bFromSweep :type Boolean) (SweepResult :type Hit%20Result%20Structure%20%28by%20ref%29)))

(event OnClicked(SpinReelsBox)
  (params (TouchedComponent :type Primitive%20Component%20Object%20Reference) (ButtonPressed :type Key%20Structure :default "None"))
  (bind _playercharacter (Variables|Default|GetPlayerCharacter))
  ;[1 1 1] отключаем возможность кликать мышкой
  (Rendering|SetVisibility (Variables|Default|GetRedLine) false false)
  (Variables|/Script/Engine.PlayerController|SetbEnableClickEvents (Game|GetPlayerController 0) false)
  (Utilities|FlowControl|Delay 0.3)
  (Variables|Default|SetSpeedRotation 0.018)
  (CallFunction|SlotRotation)
  ;[1 1 1] остановить вращение через 3 секунду изменив скорость вращения
  (Utilities|FlowControl|Delay 2.0)
  (Variables|Default|SetSpeedRotation 0.0)
  (Variables|Default|SetstopSlotRotation true)
  (Utilities|FlowControl|Delay 0.2)
  (CallFunction|CheckFirstReel)
  (CallFunction|CheckSecondReel)
  (CallFunction|CheckThirdReel)
  (Variables|/Script/Engine.PlayerController|SetbEnableClickEvents (Game|GetPlayerController 0) true)
  (if (== (Variables|Default|GetLemonPoints) 3)
    (Development|PrintString "LEMON + 3")
    (Variables|Default|SetLemonPoints 0)
    (Rendering|SetVisibility (Variables|Default|GetRedLine) true false)
    (Default|AddCredit (Variables|Default|GetPlayerCharacter) 3.0)
    (Default|ShowCreditChangeAnimation (Variables|/Game/Blueprint/BP_ThirdPersonCharacter.BP_ThirdPersonCharacter_C|GetCredit%20Widget (Variables|Default|GetPlayerCharacter)) "+3")
    (else
      (Default|AddCredit _playercharacter -25.0)
      (Default|ShowCreditChangeAnimation (Variables|/Game/Blueprint/BP_ThirdPersonCharacter.BP_ThirdPersonCharacter_C|GetCredit%20Widget _playercharacter) "-25")
      (Variables|Default|SetLemonPoints 0)
      (if (== (Variables|Default|GetCherryPoints) 6)
        (Development|PrintString "Cherry + 6")
        (Variables|Default|SetCherryPoints 0)
        (Rendering|SetVisibility (Variables|Default|GetRedLine) true false)
        (Default|ShowCreditChangeAnimation (Variables|/Game/Blueprint/BP_ThirdPersonCharacter.BP_ThirdPersonCharacter_C|GetCredit%20Widget (Variables|Default|GetPlayerCharacter)) "+3")
        (else
          (Variables|Default|SetCherryPoints 0)
          (if (== (Variables|Default|GetWatermelonPoints) 9)
            (Development|PrintString "Watermelon + 9")
            (Variables|Default|SetWatermelonPoints 0)
            (Rendering|SetVisibility (Variables|Default|GetRedLine) true false)
            ;[1 1 1] 25 которые снимаем в самом начале +9 за выигрыш
            (Default|AddCredit (Variables|Default|GetPlayerCharacter) 34.0)
            (Default|ShowCreditChangeAnimation (Variables|/Game/Blueprint/BP_ThirdPersonCharacter.BP_ThirdPersonCharacter_C|GetCredit%20Widget (Variables|Default|GetPlayerCharacter)) "+9")
            (else
              (Variables|Default|SetWatermelonPoints 0)
              (if (== (Variables|Default|GetPlumPoints) 15)
                (Development|PrintString "Plum +15")
                (Variables|Default|SetPlumPoints 0)
                (Rendering|SetVisibility (Variables|Default|GetRedLine) true false)
                (Default|AddCredit (Variables|Default|GetPlayerCharacter) 4e+01)
                (Default|ShowCreditChangeAnimation (Variables|/Game/Blueprint/BP_ThirdPersonCharacter.BP_ThirdPersonCharacter_C|GetCredit%20Widget (Variables|Default|GetPlayerCharacter)) "+15")
                (else
                  (Variables|Default|SetPlumPoints 0)
                  (if (== (Variables|Default|GetBarPoints) 90)
                    (Development|PrintString "Bar + 90")
                    (Variables|Default|SetBarPoints 0)
                    (Rendering|SetVisibility (Variables|Default|GetRedLine) true false)
                    (Default|AddCredit (Variables|Default|GetPlayerCharacter) 115.0)
                    (Default|ShowCreditChangeAnimation (Variables|/Game/Blueprint/BP_ThirdPersonCharacter.BP_ThirdPersonCharacter_C|GetCredit%20Widget (Variables|Default|GetPlayerCharacter)) "+90")
                    (else
                      (Variables|Default|SetBarPoints 0)
                      (if (== (Variables|Default|GetSevenPoints) 777)
                        (Development|PrintString "SEVEN +777")
                        (Variables|Default|SetSevenPoints 0)
                        (Rendering|SetVisibility (Variables|Default|GetRedLine) true false)
                        (Default|AddCredit (Variables|Default|GetPlayerCharacter) 802.0)
                        (Default|ShowCreditChangeAnimation (Variables|/Game/Blueprint/BP_ThirdPersonCharacter.BP_ThirdPersonCharacter_C|GetCredit%20Widget (Variables|Default|GetPlayerCharacter)) "+777")
                        (else
                          (Variables|Default|SetSevenPoints 0)
                          (Development|PrintString "YOU LOSE 25"))))))))))))))

(event OnComponentBeginOverlap(CheckSlotBoxSecondReel)
  (params (OverlappedComponent :type Primitive%20Component%20Object%20Reference) (OtherActor :type Actor%20Object%20Reference) (OtherComp :type Primitive%20Component%20Object%20Reference) (OtherBodyIndex :type Integer) (bFromSweep :type Boolean) (SweepResult :type Hit%20Result%20Structure%20%28by%20ref%29)))

(event OnComponentBeginOverlap(CheckSlotBoxThirdReel)
  (params (OverlappedComponent :type Primitive%20Component%20Object%20Reference) (OtherActor :type Actor%20Object%20Reference) (OtherComp :type Primitive%20Component%20Object%20Reference) (OtherBodyIndex :type Integer) (bFromSweep :type Boolean) (SweepResult :type Hit%20Result%20Structure%20%28by%20ref%29)))

(event OnComponentBeginOverlap(Box)
  (params (OverlappedComponent :type Primitive%20Component%20Object%20Reference) (OtherActor :type Actor%20Object%20Reference) (OtherComp :type Primitive%20Component%20Object%20Reference) (OtherBodyIndex :type Integer) (bFromSweep :type Boolean) (SweepResult :type Hit%20Result%20Structure%20%28by%20ref%29))
  (bind _textpresse (Variables|Default|GetTextPressE))
  ;[1 1 1] вертим текст в стороун персонажа
  (Rendering|SetVisibility (Variables|Default|GetTextPressE) true false)
  (Variables|Default|SetcanUseSlotMachine true)
  (Transformation|SetWorldRotation _textpresse (Math|Rotator|FindLookatRotation (Transformation|GetWorldLocation _textpresse) (Transformation|GetWorldLocation (Variables|/Script/Engine.Actor|GetRootComponent (Game|GetPlayerCameraManager 0)))) false false))

(event OnComponentEndOverlap(Box)
  (params (OverlappedComponent :type Primitive%20Component%20Object%20Reference) (OtherActor :type Actor%20Object%20Reference) (OtherComp :type Primitive%20Component%20Object%20Reference) (OtherBodyIndex :type Integer))
  (Rendering|SetVisibility (Variables|Default|GetTextPressE) false false)
  (Variables|Default|SetcanUseSlotMachine false))

(event OnEndCursorOver(MaxCreditBox)
  (params (TouchedComponent :type Primitive%20Component%20Object%20Reference))
  ;[1 1 1] On Begin Cursor Over работает с Box Collision только если Collision Presets - BlockAllDinamic
  (Rendering|SetVisibility (Variables|Default|GetRectLightMaxCredit) false false))

(event OnBeginCursorOver(SpinReelsBox)
  (params (TouchedComponent :type Primitive%20Component%20Object%20Reference))
  (Rendering|SetVisibility (Variables|Default|GetRectLightSpinReels) true false))

(event OnEndCursorOver(SpinReelsBox)
  (params (TouchedComponent :type Primitive%20Component%20Object%20Reference))
  (Rendering|SetVisibility (Variables|Default|GetRectLightSpinReels) false false))

(event OnBeginCursorOver(BetOneBox)
  (params (TouchedComponent :type Primitive%20Component%20Object%20Reference))
  (Rendering|SetVisibility (Variables|Default|GetRectLightBetOne) true false))

(event OnEndCursorOver(BetOneBox)
  (params (TouchedComponent :type Primitive%20Component%20Object%20Reference))
  (Rendering|SetVisibility (Variables|Default|GetRectLightBetOne) false false))

(event OnBeginCursorOver(CashOutBox)
  (params (TouchedComponent :type Primitive%20Component%20Object%20Reference))
  (Rendering|SetVisibility (Variables|Default|GetRectLightCashOut) true false))

(event Custom|CheckThirdReel
  (Utilities|Time|SetTimerbyEvent (delegate Custom|CheckThirdReel) 0.0)
  (for _array_element (Variables|/Script/Engine.ActorComponent|GetComponentTags (stale OnComponentBeginOverlap(CheckSlotBoxThirdReel) OtherComp))
    (switch string (Utilities|String|ToString(Name) _array_element)
      (:Lemon
        (Variables|Default|SetLemonPoints (+ (Variables|Default|GetLemonPoints) 1)))
      (:Cherry
        (Variables|Default|SetCherryPoints (+ (Variables|Default|GetCherryPoints) 2)))
      (:Watermelon
        (Variables|Default|SetWatermelonPoints (+ 3 (Variables|Default|GetWatermelonPoints))))
      (:Plum
        (Variables|Default|SetPlumPoints (+ 5 (Variables|Default|GetPlumPoints))))
      (:Bar
        (Variables|Default|SetBarPoints (+ 30 (Variables|Default|GetBarPoints))))
      (:Seven
        (Variables|Default|SetSevenPoints (+ 259 (Variables|Default|GetSevenPoints)))))))

(event Custom|SlotRotation
  ;[1 1 1] случайно вертим три барабана с случайной(select) скоростью
  (Utilities|Time|SetTimerbyEvent (delegate Custom|SlotRotation) (Variables|Default|GetSpeedRotation) true)
  (Transformation|AddLocalRotation (Variables|Default|GetFirstReel) (Math|Rotator|MakeRotator (Utilities|Select :Index (Math|Random|RandomIntegerinRange 0 14) :Option%200 18.0 :Option%201 36.0 :Option%202 54.0 :Option%203 72.0 :Option%204 9e+01 :Option%205 108.0 :Option%206 126.0 :Option%207 144.0 :Option%208 162.0 :Option%209 1.8e+02 :Option%2010 198.0 :Option%2011 216.0 :Option%2012 234.0 :Option%2013 252.0 :Option%2014 2.7e+02) 0.0 0.0) false false)
  (Transformation|AddLocalRotation (Variables|Default|GetSecondReel) (Math|Rotator|MakeRotator (Utilities|Select :Index (Math|Random|RandomIntegerinRange 0 14) :Option%200 18.0 :Option%201 36.0 :Option%202 54.0 :Option%203 72.0 :Option%204 9e+01 :Option%205 108.0 :Option%206 126.0 :Option%207 144.0 :Option%208 162.0 :Option%209 1.8e+02 :Option%2010 198.0 :Option%2011 216.0 :Option%2012 234.0 :Option%2013 252.0 :Option%2014 2.7e+02) 0.0 0.0) false false)
  (Transformation|AddLocalRotation (Variables|Default|GetThirdReel) (Math|Rotator|MakeRotator (Utilities|Select :Index (Math|Random|RandomIntegerinRange 0 14) :Option%200 18.0 :Option%201 36.0 :Option%202 54.0 :Option%203 72.0 :Option%204 9e+01 :Option%205 108.0 :Option%206 126.0 :Option%207 144.0 :Option%208 162.0 :Option%209 1.8e+02 :Option%2010 198.0 :Option%2011 216.0 :Option%2012 234.0 :Option%2013 252.0 :Option%2014 2.7e+02) 0.0 0.0) false false))

(event Custom|GetCameraRoulleteAfterPlay)

(event Custom|CheckFirstReel
  (Utilities|Time|SetTimerbyEvent (delegate Custom|CheckFirstReel) 0.0)
  (for _array_element (Variables|/Script/Engine.ActorComponent|GetComponentTags (stale OnComponentBeginOverlap(CheckSlotBoxFirstReel) OtherComp))
    (switch string (Utilities|String|ToString(Name) _array_element)
      (:Lemon
        ;[1 1 1] дает за кажыдй лимон в барабане по 1 очку. если общее количество очков не равно 3 это значит что выигрыша нет так как дял выигрыша нужно все 3 фигурки
        (Variables|Default|SetLemonPoints (+ (Variables|Default|GetLemonPoints) 1)))
      (:Cherry
        (Variables|Default|SetCherryPoints (+ (Variables|Default|GetCherryPoints) 2)))
      (:Watermelon
        (Variables|Default|SetWatermelonPoints (+ 3 (Variables|Default|GetWatermelonPoints))))
      (:Plum
        (Variables|Default|SetPlumPoints (+ 5 (Variables|Default|GetPlumPoints))))
      (:Bar
        (Variables|Default|SetBarPoints (+ 30 (Variables|Default|GetBarPoints))))
      (:Seven
        (Variables|Default|SetSevenPoints (+ 259 (Variables|Default|GetSevenPoints)))))))

(event Custom|CheckSecondReel
  (Utilities|Time|SetTimerbyEvent (delegate Custom|CheckSecondReel) 0.0)
  (for _array_element (Variables|/Script/Engine.ActorComponent|GetComponentTags (stale OnComponentBeginOverlap(CheckSlotBoxSecondReel) OtherComp))
    (switch string (Utilities|String|ToString(Name) _array_element)
      (:Lemon
        (Variables|Default|SetLemonPoints (+ (Variables|Default|GetLemonPoints) 1)))
      (:Cherry
        (Variables|Default|SetCherryPoints (+ (Variables|Default|GetCherryPoints) 2)))
      (:Watermelon
        (Variables|Default|SetWatermelonPoints (+ 3 (Variables|Default|GetWatermelonPoints))))
      (:Plum
        (Variables|Default|SetPlumPoints (+ 5 (Variables|Default|GetPlumPoints))))
      (:Bar
        (Variables|Default|SetBarPoints (+ 30 (Variables|Default|GetBarPoints))))
      (:Seven
        (Variables|Default|SetSevenPoints (+ 259 (Variables|Default|GetSevenPoints)))))))

(event EventBeginPlay
  (bind _asbp_third_person_character (Utilities|Casting|CastToBP_ThirdPersonCharacter (Game|Player|GetPlayerPawn 0)))
  ;[1 1 1] Включаем ActionInput
  (Variables|Default|SetPlayerCharacter _asbp_third_person_character)
  (Input|EnableInput (Game|GetPlayerController 0))
  ;[1 1 1] Иначе Event с мышкйо не работают
  (Variables|/Script/Engine.PlayerController|SetbEnableMouseOverEvents (Game|GetPlayerController 0) true)
  ;[1 1 1] Иначе клики не работают
  (Variables|/Script/Engine.PlayerController|SetbEnableClickEvents (Game|GetPlayerController 0) true)
  (Rendering|SetVisibility (Variables|Default|GetRedLine) false false)
  (Rendering|SetVisibility (Variables|Default|GetTextPressE) false false))

(event Input|KeyboardEvents|E
  (params (Key :type Key%20Structure :default "None"))
  ;[1 1 1] Что бы работало нужен EnableInput в Beginplay
  ; Для того что бы исспользовать одну клавишу E в разных местах я отключил тут ConsumeInput
)

(event Input|KeyboardEvents|E
  (params (Key :type Key%20Structure :default "None"))
  (bind _playercharacter (Variables|Default|GetPlayerCharacter))
  (:Pressed
    (if (Variables|Default|GetcanUseSlotMachine)
      (Default|GetCameraSlotMachine (Variables|Default|GetPlayerCharacter))
      (Transformation|AddActorWorldOffset _playercharacter (Utilities|Operators|Subtract (Transformation|GetActorLocation self) (Transformation|GetActorLocation _playercharacter) "110.000000,0.000000,0.000000"))
      (Transformation|SetActorRelativeRotation _playercharacter)
      (Variables|Default|SetcharacterNowUseMachine true))))

(fn ConstructionScript)