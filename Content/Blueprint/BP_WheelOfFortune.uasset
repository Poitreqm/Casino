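; Wheel of fortune actor that the player spins with F inside its trigger box to win or lose credits.
; A self-re-arming timer rotates the wheel by random steps for about four seconds.
; CheckWheel maps the name of the box overlapping the arrow to points, which WhichBoxIsIt applies to the character's credit and widget animation.
; The +150 box stores -150, which the payout step does not handle.
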(event OnComponentBeginOverlap(Box)
  (params (OverlappedComponent :type Primitive%20Component%20Object%20Reference) (OtherActor :type Actor%20Object%20Reference) (OtherComp :type Primitive%20Component%20Object%20Reference) (OtherBodyIndex :type Integer) (bFromSweep :type Boolean) (SweepResult :type Hit%20Result%20Structure%20%28by%20ref%29))
  (Variables|Default|SetcanUseSlotWheel true))

(event OnComponentEndOverlap(Box)
  (params (OverlappedComponent :type Primitive%20Component%20Object%20Reference) (OtherActor :type Actor%20Object%20Reference) (OtherComp :type Primitive%20Component%20Object%20Reference) (OtherBodyIndex :type Integer))
  (Variables|Default|SetcanUseSlotWheel false))

(event OnComponentBeginOverlap(BoxArrow)
  (params (OverlappedComponent :type Primitive%20Component%20Object%20Reference) (OtherActor :type Actor%20Object%20Reference) (OtherComp :type Primitive%20Component%20Object%20Reference) (OtherBodyIndex :type Integer) (bFromSweep :type Boolean) (SweepResult :type Hit%20Result%20Structure%20%28by%20ref%29)))

(event Custom|SlotRotation
  (Utilities|Time|SetTimerbyEvent (delegate Custom|SlotRotation) (Variables|Default|GetSpeedRotation) true)
  (Transformation|AddLocalRotation (Variables|Default|Getwheel) (Math|Rotator|MakeRotator 0.0 (Utilities|Select :Index (Math|Random|RandomIntegerinRange 0 11) :Option%200 3.5 :Option%201 4.5 :Option%202 5.5 :Option%203 6.5 :Option%204 7.5 :Option%205 8.5 :Option%206 9.5 :Option%207 10.5 :Option%208 11.5 :Option%209 12.5 :Option%2010 13.5 :Option%2011 14.5) 0.0) false false))

(event Custom|CheckWheel
  (Utilities|Time|SetTimerbyEvent (delegate Custom|CheckWheel) 0.0)
  (Development|PrintString (Utilities|GetObjectName (stale OnComponentBeginOverlap(BoxArrow) OtherComp)))
  (switch string (Utilities|GetObjectName (stale OnComponentBeginOverlap(BoxArrow) OtherComp))
    (:Box+150
      (Variables|Default|SetWheelPoints -150))
    (:Box-200
      (Variables|Default|SetWheelPoints -200))
    (:Box-60
      (Variables|Default|SetWheelPoints -60))
    (:Box+25
      (Variables|Default|SetWheelPoints 25))
    (:Box+40
      (Variables|Default|SetWheelPoints 40))
    (:Box-25
      (Variables|Default|SetWheelPoints -25))
    (:Box0
      (Variables|Default|SetWheelPoints 0))
    (:Box+100
      (Variables|Default|SetWheelPoints 100))))

(event Custom|WhichBoxIsIt
  (if (== (Variables|Default|GetWheelPoints) 0)
    (Variables|Default|SetWheelPoints 0)
    (elif (== (Variables|Default|GetWheelPoints) 150)
      (Default|AddCredit (Variables|Default|GetPlayerCharacter) 1.5e+02)
      (Default|ShowCreditChangeAnimation (Variables|/Game/Blueprint/BP_ThirdPersonCharacter.BP_ThirdPersonCharacter_C|GetCredit%20Widget (Variables|Default|GetPlayerCharacter)) "+150")
      (Variables|Default|SetWheelPoints 0)
      (elif (== (Variables|Default|GetWheelPoints) -200)
        (Default|AddCredit (Variables|Default|GetPlayerCharacter) -2e+02)
        (Default|ShowCreditChangeAnimation (Variables|/Game/Blueprint/BP_ThirdPersonCharacter.BP_ThirdPersonCharacter_C|GetCredit%20Widget (Variables|Default|GetPlayerCharacter)) "-200")
        (Variables|Default|SetWheelPoints 0)
        (elif (== (Variables|Default|GetWheelPoints) -60)
          (Default|AddCredit (Variables|Default|GetPlayerCharacter) -6e+01)
          (Default|ShowCreditChangeAnimation (Variables|/Game/Blueprint/BP_ThirdPersonCharacter.BP_ThirdPersonCharacter_C|GetCredit%20Widget (Variables|Default|GetPlayerCharacter)) "-60")
          (Variables|Default|SetWheelPoints 0)
          (elif (== (Variables|Default|GetWheelPoints) 25)
            (Default|AddCredit (Variables|Default|GetPlayerCharacter) 25.0)
            (Default|ShowCreditChangeAnimation (Variables|/Game/Blueprint/BP_ThirdPersonCharacter.BP_ThirdPersonCharacter_C|GetCredit%20Widget (Variables|Default|GetPlayerCharacter)) "+25")
            (Variables|Default|SetWheelPoints 0)
            (elif (== (Variables|Default|GetWheelPoints) 40)
              (Default|AddCredit (Variables|Default|GetPlayerCharacter) 4e+01)
              (Default|ShowCreditChangeAnimation (Variables|/Game/Blueprint/BP_ThirdPersonCharacter.BP_ThirdPersonCharacter_C|GetCredit%20Widget (Variables|Default|GetPlayerCharacter)) "+40")
              (Variables|Default|SetWheelPoints 0)
              (elif (== (Variables|Default|GetWheelPoints) -25)
                (Default|AddCredit (Variables|Default|GetPlayerCharacter) -25.0)
                (Default|ShowCreditChangeAnimation (Variables|/Game/Blueprint/BP_ThirdPersonCharacter.BP_ThirdPersonCharacter_C|GetCredit%20Widget (Variables|Default|GetPlayerCharacter)) "-25")
                (Variables|Default|SetWheelPoints 0)
                (elif (== (Variables|Default|GetWheelPoints) 100)
                  (Default|AddCredit (Variables|Default|GetPlayerCharacter) 1e+02)
                  (Default|ShowCreditChangeAnimation (Variables|/Game/Blueprint/BP_ThirdPersonCharacter.BP_ThirdPersonCharacter_C|GetCredit%20Widget (Variables|Default|GetPlayerCharacter)) "+100")
                  (Variables|Default|SetWheelPoints 0))))))))))

(event EventBeginPlay
  (Input|EnableInput (Game|GetPlayerController 0))
  (Variables|/Script/Engine.PlayerController|SetbEnableMouseOverEvents (Game|GetPlayerController 0) true)
  (Variables|/Script/Engine.PlayerController|SetbEnableClickEvents (Game|GetPlayerController 0) true)
  (bind _asbp_third_person_character (Utilities|Casting|CastToBP_ThirdPersonCharacter (Game|Player|GetPlayerPawn 0)))
  (Variables|Default|SetPlayerCharacter _asbp_third_person_character))

(event Collision|EventActorBeginOverlap
  (params (OtherActor :type Actor%20Object%20Reference)))

(event EventTick
  (params (DeltaSeconds :type Float%20%28single-precision%29)))

(event Input|KeyboardEvents|F
  (params (Key :type Key%20Structure :default "None"))
  (:Pressed
    (Input|DisableInput (Game|GetPlayerController 0))
    (Utilities|FlowControl|Delay 0.3)
    (if (Variables|Default|GetcanUseSlotWheel)
      (Variables|Default|SetSpeedRotation 1e-05)
      (CallFunction|SlotRotation)
      (Utilities|FlowControl|Delay 4.0)
      (Variables|Default|SetSpeedRotation 0.0)
      (Utilities|FlowControl|Delay 0.5)
      (CallFunction|CheckWheel)
      (CallFunction|WhichBoxIsIt)
      (Input|EnableInput (Game|GetPlayerController 0)))))

(fn ConstructionScript)